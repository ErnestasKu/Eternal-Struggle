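; BP_Enemy is an enemy that chases the first player character once PawnSensing spots a pawn, using AIMoveTo.
; Mesh hits from Bullet-tagged BP_FirstPersonProjectile actors subtract the projectile's Damage from Health.
; UpdateHealthBar feeds MaxHealth divided by Health to the WB_EnemyHealthBar widget, hiding it at full health.
; At zero or lower Health, Die disables capsule collision and ragdolls the mesh through physics simulation.
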(event OnSeePawn(PawnSensing)
  (params (Pawn :type Pawn%20Object%20Reference))
  (CallFunction|FollowPawn))

(event OnComponentHit(Mesh)
  (params (HitComponent :type Primitive%20Component%20Object%20Reference) (OtherActor :type Actor%20Object%20Reference) (OtherComp :type Primitive%20Component%20Object%20Reference) (NormalImpulse :type Vector :default "0, 0, 0") (Hit :type Hit%20Result%20Structure%20%28by%20ref%29))
  (if (Actor|ActorHasTag OtherActor "Bullet")
    (bind _asbp_first_person_projectile (Utilities|Casting|CastToBP_FirstPersonProjectile OtherActor))
    (CallFunction|TakeDamage (Variables|/Game/FirstPerson/Blueprints/BP_FirstPersonProjectile.BP_FirstPersonProjectile_C|GetDamage _asbp_first_person_projectile))))

(event Custom|FollowPawn
  (AI|AIMoveTo self "0, 0, 0" (Game|GetPlayerCharacter 0) 5.0 false))

(event Custom|Ragdoll
  (bind _mesh (Variables|Character|GetMesh))
  (if (Utilities|IsValid _mesh)
    (Collision|SetCollisionEnabled _mesh "QueryAndPhysics")
    (Physics|SetSimulatePhysics _mesh true)
    (Class|SkeletalMeshComponent|SetPhysicsBlendWeight _mesh 1.0)))

(event EventBeginPlay
  (Variables|Default|SetHealth (Variables|Default|GetMaxHealth))
  (CallFunction|UpdateHealthBar))

(fn ConstructionScript)

(fn UpdateHealthBar
  (bind _healthbar (Variables|Default|GetHealthBar))
  (bind _aswb_enemy_health_bar (Utilities|Casting|CastToWB_EnemyHealthBar (UserInterface|GetUserWidgetObject (Variables|Default|GetHealthBar))))
  (Variables|/Game/Enemy/Blueprints/WB_EnemyHealthBar.WB_EnemyHealthBar_C|SetHealth _aswb_enemy_health_bar (/ (Variables|Default|GetMaxHealth) (Variables|Default|GetHealth)))
  (if (== (/ (Variables|Default|GetMaxHealth) (Variables|Default|GetHealth)) 1.0)
    (Rendering|SetVisibility _healthbar false false)
    (else
      (Rendering|SetVisibility _healthbar true false)))
  (return))

(fn TakeDamage
  (params (Damage :type Float%20%28double-precision%29))
  (bind _output_get (Variables|Default|SetHealth (- (Variables|Default|GetHealth) Damage)))
  (CallFunction|UpdateHealthBar)
  (if (<= _output_get 0.0)
    (CallFunction|Die)))

(fn Die
  (Collision|SetCollisionEnabled (Variables|Collision|GetCapsuleComponent) "NoCollision")
  (CallFunction|Ragdoll))